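; BP_GAMECONTROLLER runs an aim-and-score game, owning the UI, the shot angle and the score.
; BeginPlay creates BP_UI and caches the level's BP_方向箭頭 direction arrow.
; Ongamestartevent plays a timeline whose track sweeps 射擊角度 (shot angle) across a yaw range, rotating the arrow and filling the UI progress bar in sync.
; 碰到得分區 (score zone touched) adds fixed points to 分數 and prints the total.
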(event Custom|Ongamestartevent
  (bind _newtrack_0 (Timeline|Timeline Play)
    (:Update
      (bind _output_get (Variables|Default|Set射擊角度 (Math|Float|Lerp -6e+01 6e+01 _newtrack_0)))
      (Transformation|SetActorRotation (Variables|Default|Get方向箭頭) (Math|Rotator|MakeRotator 0.0 0.0 _output_get))
      (Progress|SetPercent (Variables|/Game/BP_UI.BP_UI_C|GetProgressBar_0 (Variables|Default|GetUI)) _newtrack_0))))

(event Custom|碰到得分區
  (Development|PrintString "觸發得分區事件")
  (bind _output_get (Variables|Default|Set分數 (+ (Variables|Default|Get分數) 5)))
  (Development|PrintString (Utilities|String|Append "目前得分" (Utilities|String|ToString(Text) (Utilities|Text|ToText(Integer) _output_get)))))

(event EventBeginPlay
  (Development|PrintString "GAME START")
  (bind _returnvalue (UserInterface|CreateWidget "/Game/BP_UI.BP_UI_C"))
  (Variables|Default|SetUI _returnvalue)
  (UserInterface|Viewport|AddtoViewport _returnvalue 0)
  (bind _returnvalue_2 (Actor|GetActorOfClass "/Game/BP_方向箭頭.BP_方向箭頭_C"))
  (Variables|Default|Set方向箭頭 _returnvalue_2))

(event EventTick
  (params (DeltaSeconds :type Float%20%28single-precision%29)))

(fn ConstructionScript)